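; Interactable lore object that grants its LoreItemID through the player's BP_LoreInteractor, optionally teaching emotes and feats, adding an inventory item and showing a lore popup.
; BeginPlay loads row data, image and sound from LoreObjectsTable, then hides already-collected game items on non-dedicated instances, polling until the player character exists.
; Activation gates repeat grants on Canbeusedagain, checks feat prerequisites and logs an Exiles Journey event.
; Box overlap shows a cooldown-limited interact prompt to the local player.
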(event OnComponentBeginOverlap(Box)
  (params (OverlappedComponent :type Primitive%20Component%20Object%20Reference) (OtherActor :type Actor%20Object%20Reference) (OtherComp :type Primitive%20Component%20Object%20Reference) (OtherBodyIndex :type Integer) (bFromSweep :type Boolean) (SweepResult :type Hit%20Result%20Structure%20%28by%20ref%29))
  (bind _returnvalue (Actor|GetComponentsByClass OtherActor "/Game/Systems/Components/PlayerNotificationComponent.PlayerNotificationComponent_C"))
  (bind _returnvalue_2 (Actor|GetComponentsByClass OtherActor "/Game/Items/LoreObjects/BP_LoreInteractor.BP_LoreInteractor_C"))
  (bind _item (Utilities|Array|Get(acopy) _returnvalue))
  (if (> (Utilities|Array|Length _returnvalue) 0)
    (if (not (Variables|/Game/Systems/Components/PlayerNotificationComponent.PlayerNotificationComponent_C|GetInteractNotificationCooldownInProgress _item))
      (Variables|Default|SetPlayerNotificationComponent _item)
      (Utilities|FlowControl|DoOnce false
        (:Completed
          (if (Variables|Default|GetDisplayInteractionText)
            (if (> (Utilities|Array|Length _returnvalue_2) 0)
              (bind _returnvalue_3 (Default|HasLoreItem (Utilities|Array|Get(acopy) _returnvalue_2) (Variables|Default|GetLoreItemID)))
              (if (not _returnvalue_3)
                (bind _asconan_character (Utilities|Casting|CastToConanCharacter OtherActor))
                (bind _isremoteactor (CallFunction|IsRemoteActor _asconan_character))
                (if (not _isremoteactor)
                  (CallFunction|ClientShowNotification _asconan_character)
                  (Default|StartInteractNotificationCooldown (Variables|Default|GetPlayerNotificationComponent)))))
            (else
              (bind _asconan_character_2 (Utilities|Casting|CastToConanCharacter OtherActor))
              (bind _isremoteactor_2 (CallFunction|IsRemoteActor _asconan_character_2))
              (if (not _isremoteactor_2)
                (CallFunction|ClientShowNotification _asconan_character_2)
                (Default|StartInteractNotificationCooldown (Variables|Default|GetPlayerNotificationComponent))))))))))

(event Custom|ClientShowNotification
  (params (Character :type Conan%20Character%20Object%20Reference))
  (bind _returnvalue (Game|GetPlayerController 0))
  (bind _ashudinterface (Utilities|Casting|CastToHUDInterface (HUD|GetHUD _returnvalue)))
  (bind _returnvalue_2 (UserInterface|CreateWidget "/Game/UI/HUD/Notifications/W_ActionTutorial.W_ActionTutorial_C" _returnvalue))
  (Class|ActionTutorial|CreateActionTutorial _returnvalue_2 "PRESS {0} TO INTERACT" "InteractKey")
  (Class|ActionTutorial|SetFont _returnvalue_2 (Utilities|Struct|MakeSlateFontInfo "/Game/Slate/KelsonSans.KelsonSans" 0 "(OutlineSize=0,OutlineMaterial=None,OutlineColor=(R=0.000000,G=0.000000,B=0.000000,A=1.000000),bSeparateFillAlpha=False)" "Normal" 16))
  (Default|ShowCustomWidgetNotification _ashudinterface _returnvalue_2))

(event Custom|Teach%20Multiple%20Emotes
  (params (Emote%20Controller :type BP%20Emote%20Controller%20Object%20Reference))
  (bind _emotetolearn (Variables|Default|GetEmoteToLearn))
  (if (> (Utilities|Array|Length (Variables|Default|GetEmote%20list%20to%20learn)) 0)
    (for _array_element (Variables|Default|GetEmote%20list%20to%20learn)
      (Class|EmoteController|LearnEmote Emote%20Controller _array_element)
      (if (Networking|IsServer)
        (Class|ConanCharacter|ClientHUDShowNotification (.AsConan%20Character (Utilities|Casting|CastToConanCharacter (Pawn|GetControlledPawn (stale EventInteractableActivate Instigator)))) (Utilities|Text|FormatText "Learned {\"0\"}!" (Utilities|Text|ToText(String) (Utilities|String|EnumtoString _array_element))) false)))
    (else
      (Class|EmoteController|LearnEmote Emote%20Controller _emotetolearn)
      (if (and (Networking|IsServer) (Utilities|Enum|NotEqual(Enum) _emotetolearn "None"))
        (Class|ConanCharacter|ClientHUDShowNotification (.AsConan%20Character (Utilities|Casting|CastToConanCharacter (Pawn|GetControlledPawn (stale EventInteractableActivate Instigator)))) (Utilities|Text|FormatText "Learned {\"0\"}!" (Utilities|Text|ToText(String) (Utilities|String|EnumtoString _emotetolearn))) false)))))

(event EventBeginPlay
  (bind _returnvalue (Game|GetPlayerCharacter 0))
  (bind _returnvalue_2 (Actor|GetComponentsByClass _returnvalue "/Game/Items/LoreObjects/BP_LoreInteractor.BP_LoreInteractor_C"))
  (bind _returnvalue_3 (Utilities|GetDataTableRow "/Game/Items/LoreObjects/LoreObjectsTable.LoreObjectsTable" (Utilities|String|StringToName (Utilities|String|ToString(Integer) (Variables|Default|GetLoreItemID))))
    (:then
      (bind _output_get (Variables|Default|SetLoreInfo _returnvalue_3))
      (bind _object (Utilities|AsyncLoadAsset (.Image (Utilities|Struct|BreakLoreInfo _output_get))))
      (Variables|Default|SetLoreImage _object)
      (bind _object_2 (Utilities|AsyncLoadAsset (.Sound (Utilities|Struct|BreakLoreInfo _output_get))))
      (Variables|Default|SetLoreSound _object_2)
      (if (.IsGameItem (Utilities|Struct|BreakLoreInfo _output_get))
        ;[1 1 1] This should probably be set up to get a message when the character is ready
        (if (not (Networking|IsDedicatedServer))
          (Utilities|IsValid _returnvalue :!label _label
            (:Is%20Valid
              (if (> (Utilities|Array|Length _returnvalue_2) 0)
                (bind _returnvalue_4 (Default|HasLoreItem (Utilities|Array|Get(acopy) _returnvalue_2) (Variables|Default|GetLoreItemID)))
                (if _returnvalue_4
                  (CallFunction|Hideme))))
            (:Is%20Not%20Valid
              (Utilities|FlowControl|Delay 0.5)
              (goto _label))))))
    (:RowNotFound
      (Utilities|DebugPrint :DebugLevel "INFOL_DATAERROR" :LogChannel "Items" :Duration 1e+01 :Key "BP_interactable_clientside_C"))))

(event EventInteractableActivate
  (params (Component :type Primitive%20Component%20Object%20Reference) (Instigator :type Player%20Controller%20Object%20Reference) (HitIndex :type Integer))
  (bind _returnvalue (Pawn|GetControlledPawn Instigator))
  (bind _returnvalue_2 (Pawn|GetControlledPawn Instigator))
  (bind _loreitemid (Variables|Default|GetLoreItemID))
  (bind _featstolearn (Variables|Default|GetFeatsToLearn))
  (bind _returnvalue_3 (Actor|GetComponentsByClass _returnvalue_2 "/Game/Characters/Emotes/BPEmoteController.BPEmoteController_C"))
  (bind _returnvalue_4 (Actor|GetComponentsByClass _returnvalue_2 "/Game/Items/LoreObjects/BP_LoreInteractor.BP_LoreInteractor_C"))
  (bind _asconan_character (Utilities|Casting|CastToConanCharacter _returnvalue))
  (bind _item (Utilities|Array|Get(acopy) _returnvalue_4))
  (Utilities|FlowControl|Sequence
    (:then_0
      (if (> (Utilities|Array|Length _returnvalue_4) 0)
        (bind _returnvalue_5 (Default|HasLoreItem _item (Variables|Default|GetLoreItemID)))
        (if _returnvalue_5
          (if (Variables|Default|GetCanbeusedagain?)
            (CallFunction|TeachMultipleEmotes (Utilities|Array|Get(acopy) _returnvalue_3) :!label _label)
            (Default|EventGiveLoreItem _item _loreitemid)
            (Default|EventLoreItemInteract _item _loreitemid self)
            (if (.IsGameItem (Utilities|Struct|BreakLoreInfo (Variables|Default|GetLoreInfo)))
              (bind _returnvalue_6 (Class|ConanCharacter|GetBackpackInventory (.AsConan%20Character (Utilities|Casting|CastToConanCharacter _returnvalue_2))))
              (Class|ItemInventory|AddItemTemplate _returnvalue_6 _loreitemid -1 1 false (Variables|Default|GetLoreitemdurability) -1.0) ; To Spawn an item with 0 - 100% durability, modify the Durability Percentage parameter and leave the Durability parameter to its default -1 value. To set a specific Durability value, change the Durability parameter from 0 - MaxDurability. (Values are caped)
            ))
          (elif (> (Utilities|Array|Length _returnvalue_3) 0)
            (goto _label)))))
    (:then_1
      ;[1 1 1] Learn Feats/Recipes
      (if (> (Utilities|Array|Length _featstolearn) 0)
        (for _array_element _featstolearn
          (bind _returnvalue_7 (Utilities|GetDataTableRow "/Game/Items/Feats/FeatTable.FeatTable" (Utilities|String|StringToName (Utilities|String|ToString(Integer) _array_element)))
            (:then
              (bind _returnvalue_8 (Class|ConanCharacter|GetFeatInventory _asconan_character))
              (Variables|Default|SetCanLearnFeat true)
              (for _array_element_2 (.PrerequisiteFeat (Utilities|Struct|BreakFeatTableRow _returnvalue_7))
                (if (not (Utilities|IsValid (Class|ItemInventory|GetItembyTemplateID _returnvalue_8 _array_element_2)))
                  (Variables|Default|SetCanLearnFeat false)))
              (if (Variables|Default|GetCanLearnFeat)
                (bind _returnvalue_9 (Class|ConanCharacter|GetProgressionSystem _asconan_character))
                (Class|ProgressionSystem|ServerForceLearnFeat _returnvalue_9 _array_element false)))))
        (if (Variables|Default|GetCanLearnFeat)
          (Class|ConanCharacter|ClientHUDShowNotification _asconan_character (Variables|Default|GetFeatLearnedFIFOText) false)
          (else
            (Class|ConanCharacter|ClientHUDShowNotification _asconan_character (Utilities|Text|MakeLiteralText "You don't have the knowledge required to learn these recipes.") false)))))
    (:then_2
      ;[1 1 1] Display Lorepopup
      (if (Variables|Default|GetDisplayLorePopup)
        (bind _asfun_combat_player_controller (Utilities|Casting|CastToFunCombat_PlayerController Instigator))
        (Default|ClientDisplayLorePopup _asfun_combat_player_controller (Variables|Default|GetLoreItemID))))
    (:then_3
      (CallFunction|ExilesJourneyEvent Instigator))))

(event Collision|EventActorEndOverlap
  (params (OtherActor :type Actor%20Object%20Reference))
  (Utilities|FlowControl|DoOnce false) ; enters at Reset
)

(fn ConstructionScript)

(fn Hideme
  (Rendering|SetVisibility (Variables|Default|GetDefaultSceneRoot) false true))

(fn GetAudioCue
  (return (Variables|Default|GetLoreSound)))

(fn IsGameItem
  (return (.IsGameItem (Utilities|Struct|BreakLoreInfo (Variables|Default|GetLoreInfo)))))

(fn ExilesJourneyEvent
  (params (Instigator :type Player%20Controller%20Object%20Reference))
  (bind _returnvalue (Pawn|GetControlledPawn Instigator))
  (bind _returnvalue_2 (Actor|GetComponentbyClass _returnvalue "/Game/Systems/Progression/BP_AC_ExilesJourney.BP_AC_ExilesJourney_C"))
  (Utilities|IsValid _returnvalue_2
    (:Is%20Valid
      (Class|ExilesJourneyComponent|AddJourneyEvent _returnvalue_2 "FindLife" (Transformation|GetActorLocation _returnvalue)))))

(fn InteractableDefaultAction
  (return "" 0))

(fn InteractableGetRepairUIModuleName
  (return "None"))

(fn InteractableGetUIModuleName
  (return "None"))

(fn InteractableMenuDisabled
  (return false))