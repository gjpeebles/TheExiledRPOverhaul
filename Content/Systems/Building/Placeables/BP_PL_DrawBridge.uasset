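; Placeable drawbridge building piece that provides shelter, rejects placement on a box-trace overlap and is raised or lowered by a lever.
; The lever multicasts chain movement and sound, then a timeline delay flips BridgeIsRaised.
; Its RepNotify plays or reverses a timeline driving bridge meshes, cogs, cable lengths and sounds, with cables and audio skipped on dedicated servers.
; The server replicates the timeline's end positions so clients can snap to the current state.
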(event Custom|PlayHingeSound
  (params (Opening :type Boolean))
  (bind _hinge_sound (Variables|Default|GetHinge_Sound))
  ;[1 1 1] Sounds
  (if (not (Networking|IsDedicatedServer))
    (if Opening
      (if (not (Class|ConanAudioComponent|IsPlaying _hinge_sound))
        (Class|ConanAudioComponent|Play _hinge_sound 0.0))
      (elif (not (Class|ConanAudioComponent|IsPlaying (Variables|Default|GetHinge_Sound)))
        (Class|ConanAudioComponent|Play (Variables|Default|GetHinge_Sound) 0.0)))))

(event Custom|MulticastChainMovement
  (bind _location (Timeline|Timeline_1 PlayFromStart)
    (:Update
      (Transformation|SetRelativeLocation (Variables|Default|GetStaticMesh6) (+ (Variables|Default|GetLeverChainStartLoc) (* _location "0,0.000000,-16.000000")) false false))))

(event Custom|StopMainSound
  ;[1 1 1] Sounds
  (if (not (Networking|IsDedicatedServer))
    (Class|ConanAudioComponent|Stop (Variables|Default|GetMainSound))))

(event Custom|CheckMainSound
  (bind _mainsound (Variables|Default|GetMainSound))
  ;[1 1 1] Sounds
  (if (not (Networking|IsDedicatedServer))
    (if (not (Class|ConanAudioComponent|IsPlaying _mainsound))
      (Class|ConanAudioComponent|Fadein _mainsound 1.0 1.0 0.0))))

(event Custom|Raise
  (bind _timeline_0 (Variables|Default|GetTimeline_0))
  (bind _returnvalue (Components|Timeline|GetPlaybackPosition _timeline_0))
  (CallFunction|CheckMainSound)
  (bind (_direction _mesh1rot _mesh2rot _cable) (Timeline|Timeline_0 Play)
    (:Update
      (switch Utilities|FlowControl|Switch|SwitchonETimelineDirection _direction
        (:Forward
          (Variables|Default|SetIsOpening true))
        (:Backward
          (Variables|Default|SetIsOpening false)))
      (Transformation|SetRelativeRotation (Variables|Default|GetStaticMesh) (* (Variables|Default|GetRaisedRotation_Mesh1) _mesh1rot) false false)
      (Transformation|SetRelativeRotation (Variables|Default|GetStaticMesh2) (* (Variables|Default|GetRaisedRotation_Mesh2) _mesh2rot) false false)
      (Transformation|SetRelativeRotation (Variables|Default|GetCog_01) (* (Variables|Default|GetRaisedRotation_Cogs) _mesh2rot) false false)
      (Utilities|FlowControl|Sequence
        (:then_0
          (if (not (Networking|IsDedicatedServer))
            (Variables|/Script/CableComponent.CableComponent|SetCableLength (Variables|Default|GetCable) (+ (* _cable 768.0) 5.0))
            (Variables|/Script/CableComponent.CableComponent|SetCableLength (Variables|Default|GetCable1) (+ (* _cable 768.0) 5.0))))
        (:then_1
          ;[1 1 1] Save Timeline Position
          (if (Networking|IsServer)
            (if (or (== _returnvalue 0.0) (== _returnvalue (Components|Timeline|GetTimelineLength _timeline_0)))
              (Variables|Default|SetReplicatedCurrentPlaybackPosition _returnvalue))))))
    (:Finished
      (CallFunction|StopMainSound))
    (:HingeSoundTriggers
      (CallFunction|PlayHingeSound (Variables|Default|GetIsOpening)))
    (:SettleSounds
      (CallFunction|PlaySettleSound (Variables|Default|GetIsOpening)))))

(event Custom|MulticastChainSound
  ;[1 1 1] Sounds
  (if (not (Networking|IsDedicatedServer))
    (Class|ConanAudioComponent|Play (Variables|Default|GetChainAudio) 0.0)))

(event Custom|PlaySettleSound
  (params (Opened :type Boolean))
  ;[1 1 1] Sounds
  (if (not (Networking|IsDedicatedServer))
    (if Opened
      (Class|ConanAudioComponent|Play (Variables|Default|GetSettleOpen_Sound) 0.0)
      (else
        (Class|ConanAudioComponent|Play (Variables|Default|GetSettleClosed_Sound) 0.0)))))

(event Custom|Lower
  (bind _timeline_0 (Variables|Default|GetTimeline_0))
  (bind _returnvalue (Components|Timeline|GetPlaybackPosition _timeline_0))
  (CallFunction|CheckMainSound)
  (bind (_direction _mesh1rot _mesh2rot _cable) (Timeline|Timeline_0 Reverse)
    (:Update
      (switch Utilities|FlowControl|Switch|SwitchonETimelineDirection _direction
        (:Forward
          (Variables|Default|SetIsOpening true))
        (:Backward
          (Variables|Default|SetIsOpening false)))
      (Transformation|SetRelativeRotation (Variables|Default|GetStaticMesh) (* (Variables|Default|GetRaisedRotation_Mesh1) _mesh1rot) false false)
      (Transformation|SetRelativeRotation (Variables|Default|GetStaticMesh2) (* (Variables|Default|GetRaisedRotation_Mesh2) _mesh2rot) false false)
      (Transformation|SetRelativeRotation (Variables|Default|GetCog_01) (* (Variables|Default|GetRaisedRotation_Cogs) _mesh2rot) false false)
      (Utilities|FlowControl|Sequence
        (:then_0
          (if (not (Networking|IsDedicatedServer))
            (Variables|/Script/CableComponent.CableComponent|SetCableLength (Variables|Default|GetCable) (+ (* _cable 768.0) 5.0))
            (Variables|/Script/CableComponent.CableComponent|SetCableLength (Variables|Default|GetCable1) (+ (* _cable 768.0) 5.0))))
        (:then_1
          ;[1 1 1] Save Timeline Position
          (if (Networking|IsServer)
            (if (or (== _returnvalue 0.0) (== _returnvalue (Components|Timeline|GetTimelineLength _timeline_0)))
              (Variables|Default|SetReplicatedCurrentPlaybackPosition _returnvalue))))))
    (:Finished
      (CallFunction|StopMainSound))
    (:HingeSoundTriggers
      (CallFunction|PlayHingeSound (Variables|Default|GetIsOpening)))
    (:SettleSounds
      (CallFunction|PlaySettleSound (Variables|Default|GetIsOpening)))))

(event EventBeginPlay
  ;[1 1 1] Update drawbridge on relevancy
  (Utilities|FlowControl|Sequence
    (:then_0
      (if (Networking|IsDedicatedServer)
        (Components|DestroyComponent (Variables|Default|GetCable))
        (elif (not (Variables|Default|GetIsABrush))
          (Utilities|FlowControl|Delay 1.0)
          (Development|SetHiddeninGame (Variables|Default|GetCable) false false))))
    (:then_1
      (if (Networking|IsServer)
        (Components|Timeline|SetPlaybackPosition (Variables|Default|GetTimeline_0) (Variables|Default|GetReplicatedCurrentPlaybackPosition) false true)))))

(event EventInteractableActivate
  (params (Component :type Primitive%20Component%20Object%20Reference) (Instigator :type Player%20Controller%20Object%20Reference) (HitIndex :type Integer))
  (if (== Component (Variables|Default|GetLeverCollision))
    (CallFunction|MulticastChainSound)
    (CallFunction|MulticastChainMovement)
    (Timeline|Timeline_2 PlayFromStart
      (:Finished
        (if (Variables|Default|GetBridgeIsRaised)
          (Variables|Default|SetBridgeIsRaised false)
          (else
            (Variables|Default|SetBridgeIsRaised true)))))))

(fn ConstructionScript
  (|CallParentFunction)
  (Variables|Default|SetLeverChainStartLoc (Variables|/Script/Engine.SceneComponent|GetRelativeLocation (Variables|Default|GetStaticMesh6))))

(fn CanbePlaced
  (params (AttachTo :type Buildable%20Base%20Object%20Reference) (InstanceIndex :type Integer))
  (bind _collisionchecker (Variables|Components|GetCollisionChecker))
  (bind _returnvalue (Transformation|GetWorldLocation _collisionchecker))
  (bind (_failedmessage _returnvalue_2) (|CallParentFunction AttachTo InstanceIndex))
  (if (< (Math|Conversions|ToInteger(Byte) _returnvalue_2) (Math|Conversions|ToInteger(Byte) (Utilities|Enum|LiteralenumECanBePlacedResult "Fail")))
    (bind _returnvalue_3 (Collision|BoxTraceByChannel _returnvalue (- _returnvalue "0, 0,4.000000") (Variables|/Script/Engine.BoxComponent|GetBoxExtent _collisionchecker) (Transformation|GetWorldRotation _collisionchecker) "TraceTypeQuery3" false 0 "None"))
    (if _returnvalue_3
      (return "" "Fail_Overlaps")
      (else
        (return "" "Success")))
    (else
      (return _failedmessage _returnvalue_2))))

(fn OnRepBridgeIsRaised
  (if (not (Math|Boolean|Equal(Boolean) (Variables|Default|GetLastKnownBridgeIsRaised) (Variables|Default|GetBridgeIsRaised)))
    (if (Variables|Default|GetBridgeIsRaised)
      (CallFunction|Raise)
      (else
        (CallFunction|Lower)))
    (Variables|Default|SetLastKnownBridgeIsRaised (Variables|Default|GetBridgeIsRaised))))

(fn OnRepReplicatedCurrentPlaybackPosition
  (if (not (Networking|IsServer))
    (Components|Timeline|SetPlaybackPosition (Variables|Default|GetTimeline_0) (Variables|Default|GetReplicatedCurrentPlaybackPosition) false true)))

(fn ProvidesShelter
  (return true))