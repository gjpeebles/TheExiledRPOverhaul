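; Server settings Blueprint that migrates its saved config between versions, with the latest Blueprint config version set at 15.
; On UpdateBlueprintConfig it logs the upgrade, then runs a sequence of version-gated steps.
; Each step uses ShouldApplyUpgrade to check whether its version lies between old and new, then resets named NPC rotation, avoidance and targeting variables so changed defaults take effect.
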(event EventUpdateBlueprintConfig
  (params (OldVersion :type Integer) (NewVersion :type Integer))
  (Variables|UpgradeTracking|SetOldVersion OldVersion)
  (Variables|UpgradeTracking|SetNewVersion NewVersion)
  (Utilities|FlowControl|Sequence
    (:then_0
      (Utilities|DebugPrintSimple (Utilities|String|Append "Upgrading BP serversettings from version " (Utilities|String|ToString(Integer) (Variables|UpgradeTracking|GetOldVersion)) " to version " (Utilities|String|ToString(Integer) (Variables|UpgradeTracking|GetNewVersion)) ".") "INFOL_IMPORTANT" "GlobalServerChannel"))
    (:then_1
      (Utilities|ShouldApplyUpgrade 13) ; Enable Rotation Prediction by Default\nEnable Avoidance by Default\nLet NPCs get even closer before attacking
      (Class|ServerSettings|ResetVariable "RotateToTargetSendsAngularVelocity")
      (Class|ServerSettings|ResetVariable "WeaponEffectBoundsShorteningFraction")
      (Class|ServerSettings|ResetVariable "PathFollowingAvoidanceMode")
      (Class|ServerSettings|ResetVariable "TargetPredictionMaxSeconds"))
    (:then_2
      (Utilities|ShouldApplyUpgrade 14)
      (Class|ServerSettings|ResetVariable "TargetPredictionAllowSecondsForAttack"))
    (:then_3
      (Utilities|ShouldApplyUpgrade 15)
      (Class|ServerSettings|ResetVariable "RotateToTargetSendsAngularVelocity"))))

(fn ConstructionScript)

(fn GetLatestBlueprintConfigVersion
  (return 15))