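; Starving debuff component that, judging by its Damage_Percent folder, belongs to the percent-damage buff family.
; Each tick runs the parent effect, then sets the combat character's cause of death and names "starvation" as killer if health is depleted with no killer recorded.
; It then queries the owner's hunger system through its interface, clearing itself when food rises above zero or no valid hunger system exists.
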(event EventEffecttoApplyonBuffTick
  (|CallParentFunction)
  (Utilities|FlowControl|Sequence
    (:then_0
      (bind _asbase_bpcombat (Utilities|Casting|CastToBaseBPCombat (Variables|Default|GetOwningCharacter)))
      (Variables|/Game/Characters/BaseBPChar.BaseBPChar_C|SetCauseOfDeath _asbase_bpcombat "NewEnumerator1")
      (if (and (<= (Class|ConanCharacter|GetIntStat _asbase_bpcombat "HealthCurrent" "Full") 0) (Utilities|Enum|Equal(Enum) (Variables|/Script/ConanSandbox.ConanCharacter|GetkillerName _asbase_bpcombat) (Utilities|Text|MakeLiteralText "")))
        (Variables|/Script/ConanSandbox.ConanCharacter|SetkillerName _asbase_bpcombat "starvation")))
    (:then_1
      (bind _returnvalue (Class|ConanCharacter|GetHungerSystem (Variables|Default|GetOwningCharacter)))
      (Utilities|IsValid _returnvalue
        (:Is%20Valid
          (bind _asbpi_hunger_system (Utilities|Casting|CastToBPI_HungerSystem _returnvalue)
            (:then
              (bind _value (Default|GetFoodCurrent _asbpi_hunger_system))
              (if (> _value 0.0)
                (CallFunction|ClearBuff)))
            (:CastFailed
              (CallFunction|ClearBuff :!label _label))))
        (:Is%20Not%20Valid
          (goto _label))))))